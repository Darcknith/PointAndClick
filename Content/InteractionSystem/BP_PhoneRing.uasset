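; BP_PhoneRing is an interactive phone that rings on a TV event and, when answered, launches the next investigation.
; On BeginPlay it binds to the TV actor's PlayPhone dispatcher, which arms the phone and starts the ring after a delay.
; Interacting while armed runs a delay-timed sequence: ring stops, voice plays briefly, and a French text widget announces a disappearance case.
; It then calls StartLoadLevel.
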(event Custom|Phone%20ring
  (Variables|Default|Setring true)
  (Utilities|FlowControl|Delay 1.5)
  (Audio|Components|Audio|Play (Variables|Default|GetPhoneRingCue) 0.0))

(event EventBeginPlay
  (|CallParentFunction)
  (bind _returnvalue (Actor|GetActorOfClass "/Game/InteractionSystem/BP_BaseInteractiveActor_TV.BP_BaseInteractiveActor_TV_C"))
  (EventDispatchers|BindEventtoPlayPhone _returnvalue (delegate Custom|Phone%20ring))
  (Audio|Components|Audio|Stop (Variables|Default|GetPhoneRingCue)))

(event Collision|EventActorBeginOverlap
  (params (OtherActor :type Actor%20Object%20Reference))
  (|CallParentFunction OtherActor) ; This node is disabled and will not be called.\nDrag off pins to build functionality.
)

(event EventTick
  (params (DeltaSeconds :type Float%20%28single-precision%29))
  (|CallParentFunction DeltaSeconds) ; This node is disabled and will not be called.\nDrag off pins to build functionality.
)

(event EventInteract
  (bind _phonevoicecue (Variables|Default|GetPhoneVoiceCue))
  (if (Variables|Default|Getring)
    (Variables|Default|Setring false)
    (Audio|Components|Audio|Stop (Variables|Default|GetPhoneRingCue))
    (Utilities|FlowControl|Delay 0.5)
    (Audio|Components|Audio|Play _phonevoicecue 0.0)
    (Utilities|FlowControl|Delay 1.5)
    (Audio|Components|Audio|Stop _phonevoicecue)
    (bind _returnvalue (UserInterface|CreateWidget "/Game/Victorian_House/Widget/Set_Text.Set_Text_C" 0 "Une nouvelle enquete sur une dispirition, c'est partie"))
    (UserInterface|Viewport|AddtoViewport _returnvalue 0)
    (Utilities|FlowControl|Delay 2.0)
    (Widget|RemovefromParent _returnvalue)
    (Default|CallStartLoadLevel)))

(fn ConstructionScript
  (|CallParentFunction))